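; Dialogue component for the Terrarium Maker NPC, who gives a quest to supply glass bottles for terrariums, with Thai text.
; The Dialogue override switches on the active branch: introduction, Quest Accepted, then End.
; While the quest is active, it reads the remaining "Glass" trash count from BP_FirstPersonGameMode and reports it.
; At zero it thanks the player, sets GetTerra and moves to the End branch.
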(fn Dialogue
  (|CallParentFunction)
  (switch name (Variables|Default|GetActiveDialogueBranch)
    (:Default
      (bind (_state _optionindex) (CallFunction|AddDialogue "นักจัดสวนขวด" "ดอกไม้ตรงนี้สวยดีนะเนี่ย.... ว่าแต่คุณคือใครน่ะ?" (Utilities|Array|MakeArray "เพิ่งย้ายเข้ามาน่ะ")))
      (switch Utilities|FlowControl|Switch|SwitchonEnum_DialogueState _state
        (:NewEnumerator0
          (switch int _optionindex
            (:0
              (bind (_state_2 _optionindex_2) (CallFunction|AddDialogue "นักจัดสวนขวด" "งั้นหรอ ยินดีต้อนรับนะ ตอนนี้ฉันกำลังคิดอยู่ว่าจะเอาดอกไม้พวกนี้ไปทำสวนขวดดูน่ะ แต่ขวดแก้วของฉันหมดน่ะสิ" (Utilities|Array|MakeArray "เอาแก้วของฉันมั้ย? มีเยอะเลย...")))
              (switch Utilities|FlowControl|Switch|SwitchonEnum_DialogueState _state_2
                (:NewEnumerator0
                  (switch int _optionindex_2
                    (:0
                      (bind _state_3 (CallFunction|AddDialogue "นักจัดสวนขวด" "โอ้ ได้จริงๆ หรอ คุณใจดีจัง งั้นฉันขอรับน้ำใจของคุณไว้แล้วกันนะ! คุณเอาไปให้กับพนักงานเสื้อเขียวที่ร้านได้เลย เดี๋ยวฉันขอเลือกดูดอกไม้ตรงนี้ก่อนแล้วกัน                       " (Utilities|Array|MakeArray)))
                      (switch Utilities|FlowControl|Switch|SwitchonEnum_DialogueState _state_3
                        (:NewEnumerator0
                          (CallFunction|SetDialogueBranch "QuestAccepted" "NewEnumerator0")
                          (CallFunction|CloseConversation))))))))))))
    (:QuestAccepted
      (bind _asbp_first_person_game_mode (Utilities|Casting|CastToBP_FirstPersonGameMode (Game|GetGameMode)))
      (bind _trashleft (Default|GetTrashLeft _asbp_first_person_game_mode "Glass"))
      (if (== _trashleft 0)
        (bind _state_4 (CallFunction|AddDialogue "นักจัดสวนขวด" "ขอบคุณสำหรับขวดแก้วมากๆ เลยนะ ตอนนี้ฉันสามารถจัดสวนขวดกับดอกไม้พวกนี้ได้สักที!                                             " (Utilities|Array|MakeArray)))
        (switch Utilities|FlowControl|Switch|SwitchonEnum_DialogueState _state_4
          (:NewEnumerator0
            (Variables|Default|SetGetTerra? true)
            (CallFunction|SetDialogueBranch "End" "NewEnumerator0")
            (CallFunction|CloseConversation)))
        (else
          (bind _state_5 (CallFunction|AddDialogue "นักจัดสวนขวด" (Utilities|Text|FormatText "ฉันขอขวดอีกแค่ {Trash Left} ขวดก็น่าจะเพียงพอต่อการทำสวนขวดแล้วล่ะ!                       " _trashleft) (Utilities|Array|MakeArray)))
          (switch Utilities|FlowControl|Switch|SwitchonEnum_DialogueState _state_5
            (:NewEnumerator0
              (CallFunction|ClearDialogueProgress)
              (CallFunction|CloseConversation))))))
    (:End
      (bind _state_6 (CallFunction|AddDialogue "นักจัดสวนขวด" "ขอบคุณสำหรับขวดแก้วนะ เพื่อนบ้านหน้าใหม่!                    " (Utilities|Array|MakeArray)))
      (switch Utilities|FlowControl|Switch|SwitchonEnum_DialogueState _state_6
        (:NewEnumerator0
          (CallFunction|ClearDialogueProgress)
          (CallFunction|CloseConversation))))))