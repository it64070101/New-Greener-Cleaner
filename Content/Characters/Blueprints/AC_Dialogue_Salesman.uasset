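; Dialogue component for the Salesman character, who offers to sell the player tools to help with house-cleaning chores.
; Overrides the parent Dialogue function, switching on the active branch and chaining AddDialogue calls by state and option index.
; Accepting the introduction switches to the AlreadyTalk branch, while declining rolls back one progress step.
; The repeat greeting clears progress and closes on either answer, with no shop call in this graph.
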(fn Dialogue
  (|CallParentFunction)
  (switch name (Variables|Default|GetActiveDialogueBranch)
    (:Default
      (bind (_state _optionindex) (CallFunction|AddDialogue "Salesman" "Greetings! I can't help but noticed that you're cleaning your house right now, yes? " (Utilities|Array|MakeArray "Yes")))
      (switch Utilities|FlowControl|Switch|SwitchonEnum_DialogueState _state
        (:NewEnumerator0
          (switch int _optionindex
            (:0
              (bind (_state_2 _optionindex_2) (CallFunction|AddDialogue "Salesman" "Well, I might have a way to help you work more... efficiently." (Utilities|Array|MakeArray)))
              (switch Utilities|FlowControl|Switch|SwitchonEnum_DialogueState _state_2
                (:NewEnumerator0
                  (switch int _optionindex_2
                    (:0
                      (bind (_state_3 _optionindex_3) (CallFunction|AddDialogue "Salesman" "With the right price, I will sell you tools to help with your chores. What do you say, dear customer?" (Utilities|Array|MakeArray "Sure!" "Not right now")))
                      (switch Utilities|FlowControl|Switch|SwitchonEnum_DialogueState _state_3
                        (:NewEnumerator0
                          (switch int _optionindex_3
                            (:0
                              (bind _state_4 (CallFunction|AddDialogue "Salesman" "That's good to hear! Let me show you what I have to offer." (Utilities|Array|MakeArray)))
                              (switch Utilities|FlowControl|Switch|SwitchonEnum_DialogueState _state_4
                                (:NewEnumerator0
                                  (CallFunction|SetDialogueBranch "AlreadyTalk" "NewEnumerator0")
                                  (CallFunction|CloseConversation))))
                            (:1
                              (bind _state_5 (CallFunction|AddDialogue "Salesman" "Sure, stop by if you're interested." (Utilities|Array|MakeArray)))
                              (switch Utilities|FlowControl|Switch|SwitchonEnum_DialogueState _state_5
                                (:NewEnumerator0
                                  (CallFunction|RemoveDialogueProgress 1)
                                  (CallFunction|CloseConversation))))))))))))))))
    (:AlreadyTalk
      (bind (_state_6 _optionindex_4) (CallFunction|AddDialogue "Salesman" "Greetings again, dear customer! Are you interested in any of my product?" (Utilities|Array|MakeArray "Yes" "Not right now")))
      (switch Utilities|FlowControl|Switch|SwitchonEnum_DialogueState _state_6
        (:NewEnumerator0
          (switch int _optionindex_4
            (:0
              (CallFunction|ClearDialogueProgress)
              (CallFunction|CloseConversation))
            (:1
              (CallFunction|ClearDialogueProgress)
              (CallFunction|CloseConversation))))))))