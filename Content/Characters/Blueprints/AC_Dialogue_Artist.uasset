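; Dialogue component for the Artist NPC, whose Thai-language lines give the player a quest to supply waste paper for recycling into art material.
; The Dialogue override calls its parent, then selects lines by active branch: introduction, quest reminder or closing thanks.
; Single-option AddDialogue steps chain on Pass Through before closing the conversation.
; The introduction switches to QuestAccepted; nothing here sets the End branch.
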(fn Dialogue
  (|CallParentFunction)
  (switch name (Variables|Default|GetActiveDialogueBranch)
    (:Default
      (bind (_state _optionindex) (CallFunction|AddDialogue "ศิลปิน" "...สวัสดี คุณคงเป็นเพื่อนบ้านใหม่ที่เพิ่งย้ายเข้ามาใช่มั้ย? เอ่อ... ฉันขอให้คุณช่วยอะไรหน่อยได้มั้ย? คุณพอจะมีกระดาษเหลือใช้บ้างรึเปล่า? ฉันต้องการพวกมันมาทำงานศิลป์ของฉันน่ะ" (Utilities|Array|MakeArray "มีสิ!")))
      (switch Utilities|FlowControl|Switch|SwitchonEnum_DialogueState _state
        (:NewEnumerator0
          (switch int _optionindex
            (:0
              (bind _state_2 (CallFunction|AddDialogue "ศิลปิน" "ขอบคุณนะ... ถ้าคุณได้กระดาษมาแล้วก็เอาไปให้พนักงานที่ร้านซื้อขยะได้เลย เธอคนนั้นจะจัดการกับกระดาษของคุณให้กลับมาใช้ใหม่ได้อีกครั้ง เดี๋ยวฉันค่อยไปเอากระดาษที่ร้านอีกที                                                                              " (Utilities|Array|MakeArray ">")))
              (switch Utilities|FlowControl|Switch|SwitchonEnum_DialogueState _state_2
                (:NewEnumerator0
                  (CallFunction|SetDialogueBranch "QuestAccepted" "NewEnumerator0")
                  (CallFunction|CloseConversation))))))))
    (:QuestAccepted
      (bind _state_3 (CallFunction|AddDialogue "ศิลปิน" "ถ้าคุณเก็บกระดาษขายแล้วช่วยรีไซเคิลพวกมันให้ก่อนเอามาให้ฉันด้วยนะ ขอบคุณ" (Utilities|Array|MakeArray "โอเค")))
      (switch Utilities|FlowControl|Switch|SwitchonEnum_DialogueState _state_3
        (:NewEnumerator0
          (CallFunction|ClearDialogueProgress)
          (CallFunction|CloseConversation))))
    (:End
      (bind _state_4 (CallFunction|AddDialogue "ศิลปิน" "ขอบคุณสำหรับการะดาษทั้งหมดนี่นะ... ในที่สุดฉันก็จะได้ทำงานนี้ของฉันให้เสร็จได้สักที..." (Utilities|Array|MakeArray ">")))
      (switch Utilities|FlowControl|Switch|SwitchonEnum_DialogueState _state_4
        (:NewEnumerator0
          (CallFunction|ClearDialogueProgress)
          (CallFunction|CloseConversation))))))