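; Dialogue component for the waste-buyer shopkeeper NPC, who teaches waste sorting in Thai.
; Overrides Dialogue, switching on ActiveDialogueBranch and chaining AddDialogue nodes through Pass Through states and option indices.
; The default branch explains food-waste composting and RDF incineration in either order, converging on a farewell that sets AlreadyTalk and closes.
; Declining leaves the branch unchanged; AlreadyTalk gives a sorting reminder, clears progress and closes.
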(fn Dialogue
  (|CallParentFunction)
  (switch name (Variables|Default|GetActiveDialogueBranch)
    (:Default
      (bind (_state _optionindex) (CallFunction|AddDialogue "พนักงานรับซื้อขยะ" "สวัสดี คุณดูสนใจที่จะขายขยะอย่างงั้นหรือ?" (Utilities|Array|MakeArray "ใช่แล้ว" "ยังไม่สนใจตอนนี้")))
      (switch Utilities|FlowControl|Switch|SwitchonEnum_DialogueState _state
        (:NewEnumerator0
          (switch int _optionindex
            (:0
              (bind (_state_2 _optionindex_2) (CallFunction|AddDialogue "พนักงานรับซื้อขยะ" "บ้านของคุณมีขยะเยอะมาก แต่ไม่เป็นไร ฉันสามารถช่วยเรื่องจัดการขยะได้!" (Utilities|Array|MakeArray)))
              (switch Utilities|FlowControl|Switch|SwitchonEnum_DialogueState _state_2
                (:NewEnumerator0
                  (switch int _optionindex_2
                    (:0
                      (bind (_state_3 _optionindex_3) (CallFunction|AddDialogue "พนักงานรับซื้อขยะ" "ถ้าคุณมีเศษอาหาร ให้ใส่ไว้ในถังหมักปุ๋ย และถ้ามีขยะ RDF ให้เผาในเตาเผาขยะได้เลย" (Utilities|Array|MakeArray "RDF คืออะไร" "เศษอาหารคืออะไร")))
                      (switch Utilities|FlowControl|Switch|SwitchonEnum_DialogueState _state_3
                        (:NewEnumerator0
                          (switch int _optionindex_3
                            (:0
                              (bind (_state_4 _optionindex_4) (CallFunction|AddDialogue "พนักงานรับซื้อขยะ" "RDF (Refuse Derived Fuel) หรือขยะมูลฝอยเป็นขยะที่ไม่สามารถเอาไปรีไซเคิลได้เพราะถูกปนเปื้อนเยอะเกินไป จึงต้องจบด้วยการเผาทิ้งเป็นพลังงาน ซึ่งเป็นทางเลือกสุดท้ายที่เหลืออยู่! เพราะฉะนั้นถ้ารีไซเคิลได้ก็ควรรีไซเคิลดีกว่า" (Utilities|Array|MakeArray "เศษอาหารคืออะไร")))
                              (switch Utilities|FlowControl|Switch|SwitchonEnum_DialogueState _state_4
                                (:NewEnumerator0
                                  (switch int _optionindex_4
                                    (:0
                                      (bind (_state_5 _optionindex_5) (CallFunction|AddDialogue "พนักงานรับซื้อขยะ" "เศษอาหารก็คือขยะที่เกิดจากอาหารชนิดต่าง ๆ ซึ่งย่อยสลายได้ง่าย เนื่องจากเป็นสารอินทรีย์ เราจึงสามารถนำเศษอาหารที่เหลือมาผสมหมักเป็นปุ๋ยได้นั้นเอง!" (Utilities|Array|MakeArray "ขอบคุณ")))
                                      (switch Utilities|FlowControl|Switch|SwitchonEnum_DialogueState _state_5
                                        (:NewEnumerator0
                                          (switch int _optionindex_5
                                            (:0
                                              _)))))))))
                            (:1
                              (bind (_state_6 _optionindex_6) (CallFunction|AddDialogue "พนักงานรับซื้อขยะ" "เศษอาหารก็คือขยะที่เกิดจากอาหารชนิดต่าง ๆ ซึ่งย่อยสลายได้ง่าย เนื่องจากเป็นสารอินทรีย์ เราจึงสามารถนำเศษอาหารที่เหลือมาผสมหมักเป็นปุ๋ยได้นั้นเอง!" (Utilities|Array|MakeArray "RDF คืออะไร")))
                              (switch Utilities|FlowControl|Switch|SwitchonEnum_DialogueState _state_6
                                (:NewEnumerator0
                                  (switch int _optionindex_6
                                    (:0
                                      (bind (_state_7 _optionindex_7) (CallFunction|AddDialogue "พนักงานรับซื้อขยะ" "RDF (Refuse Derived Fuel) หรือขยะมูลฝอยเป็นขยะที่ไม่สามารถเอาไปรีไซเคิลได้เพราะถูกปนเปื้อนเยอะเกินไป จึงต้องจบด้วยการเผาทิ้งเป็นพลังงาน ซึ่งเป็นทางเลือกสุดท้ายที่เหลืออยู่! เพราะฉะนั้นถ้ารีไซเคิลได้ก็ควรรีไซเคิลดีกว่า" (Utilities|Array|MakeArray "ขอบคุณ")))
                                      (switch Utilities|FlowControl|Switch|SwitchonEnum_DialogueState _state_7
                                        (:NewEnumerator0
                                          (switch int _optionindex_7
                                            (:0
                                              _))))))))))
                          (bind _state_8 (CallFunction|AddDialogue "พนักงานรับซื้อขยะ" "ไม่เป็นไร ไว้เจอกันใหม่!" (Utilities|Array|MakeArray)))
                          (switch Utilities|FlowControl|Switch|SwitchonEnum_DialogueState _state_8
                            (:NewEnumerator0
                              (CallFunction|SetDialogueBranch "AlreadyTalk" "NewEnumerator0")
                              (CallFunction|CloseConversation))))))))))
            (:1
              (bind _state_9 (CallFunction|AddDialogue "พนักงานรับซื้อขยะ" "อย่างงั้นหรอ งั้นถ้าสนใจก็กลับมาคุยได้ตลอดนะ" (Utilities|Array|MakeArray)))
              (switch Utilities|FlowControl|Switch|SwitchonEnum_DialogueState _state_9))))))
    (:AlreadyTalk
      (bind _state_10 (CallFunction|AddDialogue "พนักงานรับซื้อขยะ" "คุณเก็บขยะมาใช่มั้ย? แยกขยะให้ถูกนะ! เศษอาหาร (Food Waste) ใช้ทำปุ๋ยในถังหมักปุ๋ยได้ ส่วน RDF เผาในเตาเผาขยะได้" (Utilities|Array|MakeArray)))
      (switch Utilities|FlowControl|Switch|SwitchonEnum_DialogueState _state_10
        (:NewEnumerator0
          (CallFunction|ClearDialogueProgress)
          (CallFunction|CloseConversation))))))