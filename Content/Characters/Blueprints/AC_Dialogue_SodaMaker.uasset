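; Dialogue component for the soda maker NPC, whose Thai-language quest asks the player to recycle scrap metal into cans.
; Dialogue branches run from request through QuestAccepted to End, with QuestAccepted counting game-mode recycled metal against four cans.
; On opening, it takes any soda the player holds and sets GetSoda; otherwise it jumps to End if no metal trash remains and recycling is complete, though that check queries "paper".
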(fn Dialogue
  (|CallParentFunction)
  (switch name (Variables|Default|GetActiveDialogueBranch)
    (:Default
      (bind (_state _optionindex) (CallFunction|AddDialogue "คนทำโซดาผลไม้" "สวัสดีเพื่อนบ้านหน้าใหม่!  ดูเหมือนว่าคุณกำลังยุ่งอยู่กับการทำความสะอาดบ้านอยู่สินะ พอดีฉันมีเรื่องอยากขอร้องให้คุณช่วยหน่อยน่ะ" (Utilities|Array|MakeArray "คืออะไรหรอ?")))
      (switch Utilities|FlowControl|Switch|SwitchonEnum_DialogueState _state
        (:NewEnumerator0
          (switch int _optionindex
            (:0
              (bind (_state_2 _optionindex_2) (CallFunction|AddDialogue "คนทำโซดาผลไม้" "ฉันต้องการกระป๋องเหล็กมาเพื่อใส่โซดาผลไม้เพิ่มน่ะ คุณพอจะมีให้ฉันมั้ย?" (Utilities|Array|MakeArray "เดี๋ยวดูให้นะ")))
              (switch Utilities|FlowControl|Switch|SwitchonEnum_DialogueState _state_2
                (:NewEnumerator0
                  (switch int _optionindex_2
                    (:0
                      (bind _state_3 (CallFunction|AddDialogue "คนทำโซดาผลไม้" "ขอบคุณมากๆ เลยนะสหาย! ถ้างั้นช่วยเอาขยะเหล็กที่ไม่ใช้แล้วไปขายแล้วรีไซเคิลมาให้ฉันหน่อยนะ" (Utilities|Array|MakeArray "โอเค")))
                      (switch Utilities|FlowControl|Switch|SwitchonEnum_DialogueState _state_3
                        (:NewEnumerator0
                          (CallFunction|SetDialogueBranch "QuestAccepted" "NewEnumerator0")
                          (CallFunction|CloseConversation))))))))))))
    (:QuestAccepted
      (bind (_state_4 _optionindex_3) (CallFunction|AddDialogue "คนทำโซดาผลไม้" "สวัสดีอีกครั้งสหาย! อย่าลืมรีไซเคิลเหล็กให้เป็นกระป๋องก่อนเอามาให้ฉันนะ!" (Utilities|Array|MakeArray "โอเค")))
      (switch Utilities|FlowControl|Switch|SwitchonEnum_DialogueState _state_4
        (:NewEnumerator0
          (switch int _optionindex_3
            (:0
              (bind _asbp_first_person_game_mode (Utilities|Casting|CastToBP_FirstPersonGameMode (Game|GetGameMode)))
              (if (== (- 4 (.Value (Utilities|Map|Find (Variables|/Game/FirstPerson/Blueprints/BP_FirstPersonGameMode.BP_FirstPersonGameMode_C|GetTrashRecycledMap _asbp_first_person_game_mode) "metal"))) 0)
                (CallFunction|AddDialogue "ศิลปิน" "โอ้! คุณเก็บกระป๋องครบหมดแล้ว! ขอบคุณมากๆเลยนะเพื่อน" (Utilities|Array|MakeArray "โอเค"))
                (CallFunction|SetDialogueBranch "End" "NewEnumerator0")
                (CallFunction|CloseConversation)
                (else
                  (bind _state_5 (CallFunction|AddDialogue "ศิลปิน" (Utilities|Text|FormatText "ตอนนี้ฉันยังขาดกระป๋องเหล็กอีก {metal} กระป๋อง สู้ๆ นะ" (- 4 (.Value (Utilities|Map|Find (Variables|/Game/FirstPerson/Blueprints/BP_FirstPersonGameMode.BP_FirstPersonGameMode_C|GetTrashRecycledMap _asbp_first_person_game_mode) "metal")))) (Utilities|Array|MakeArray ">")))
                  (switch Utilities|FlowControl|Switch|SwitchonEnum_DialogueState _state_5
                    (:NewEnumerator0
                      (CallFunction|ClearDialogueProgress)
                      (CallFunction|CloseConversation))))))))))
    (:End
      (bind _state_6 (CallFunction|AddDialogue "คนทำโซดาผลไม้" "ขอบคุณที่ช่วยฉันนะสหาย!                             " (Utilities|Array|MakeArray)))
      (switch Utilities|FlowControl|Switch|SwitchonEnum_DialogueState _state_6
        (:NewEnumerator0
          (CallFunction|ClearDialogueProgress)
          (CallFunction|CloseConversation))))))

(fn OpenConversation
  (bind _asbp_first_person_character (Utilities|Casting|CastToBP_FirstPersonCharacter (Game|GetPlayerCharacter 0)))
  (bind _asbp_first_person_game_mode (Utilities|Casting|CastToBP_FirstPersonGameMode (Game|GetGameMode)))
  (bind _iscomplete (Default|IsRecycleComplete _asbp_first_person_game_mode "paper"))
  (bind _trashleft (Default|GetTrashLeft _asbp_first_person_game_mode "Metal"))
  (if (Variables|/Game/FirstPerson/Blueprints/BP_FirstPersonCharacter.BP_FirstPersonCharacter_C|GetHaveSoda? _asbp_first_person_character)
    (Variables|Default|SetgetSoda? true)
    (Variables|/Game/FirstPerson/Blueprints/BP_FirstPersonCharacter.BP_FirstPersonCharacter_C|SetHaveSoda? _asbp_first_person_character false)
    (elif (and (== _trashleft 0) _iscomplete)
      (CallFunction|SetDialogueBranch "End" "NewEnumerator0")))
  (|CallParentFunction))