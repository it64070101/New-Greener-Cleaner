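; Dialogue component for the Gardener NPC, who teaches the player to compost food waste and burn RDF trash in the incinerator.
; It overrides the Dialogue function, calling the parent and switching on the active branch to chain AddDialogue lines with player options.
; The first conversation explains both waste types in the player's chosen order, then sets the AlreadyTalk branch.
; Later talks give a short sorting reminder, clear dialogue progress and close.
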(fn Dialogue
  (|CallParentFunction)
  (switch name (Variables|Default|GetActiveDialogueBranch)
    (:Default
      (bind (_state _optionindex) (CallFunction|AddDialogue "Gardener" "Hey! You just moved in here right?" (Utilities|Array|MakeArray "Yes")))
      (switch Utilities|FlowControl|Switch|SwitchonEnum_DialogueState _state
        (:NewEnumerator0
          (switch int _optionindex
            (:0
              (bind (_state_2 _optionindex_2) (CallFunction|AddDialogue "Gardener" "Your house is a big mess though... But don't worry! I can help with some of the trashes!" (Utilities|Array|MakeArray)))
              (switch Utilities|FlowControl|Switch|SwitchonEnum_DialogueState _state_2
                (:NewEnumerator0
                  (switch int _optionindex_2
                    (:0
                      (bind (_state_3 _optionindex_3) (CallFunction|AddDialogue "Gardener" "If you have any food wastes, you can dump them into my compost tumbler and if you have RDF trashes, you can burn them in the incinerator!" (Utilities|Array|MakeArray "What's an RDF trash?" "What's a food waste?")))
                      (switch Utilities|FlowControl|Switch|SwitchonEnum_DialogueState _state_3
                        (:NewEnumerator0
                          (switch int _optionindex_3
                            (:0
                              (bind (_state_4 _optionindex_4) (CallFunction|AddDialogue "Gardener" "Oh, it's a type of trashes that's hard to decompose and not really worth recycling, so we burn them for energy instead! " (Utilities|Array|MakeArray "What's a food waste?")))
                              (switch Utilities|FlowControl|Switch|SwitchonEnum_DialogueState _state_4
                                (:NewEnumerator0
                                  (switch int _optionindex_4
                                    (:0
                                      (bind (_state_5 _optionindex_5) (CallFunction|AddDialogue "Gardener" "Well, any scraps or expired food! They are easy to decompose, so we compost these wastes into fertilizers." (Utilities|Array|MakeArray "Thanks")))
                                      (switch Utilities|FlowControl|Switch|SwitchonEnum_DialogueState _state_5
                                        (:NewEnumerator0
                                          (switch int _optionindex_5
                                            (:0
                                              _)))))))))
                            (:1
                              (bind (_state_6 _optionindex_6) (CallFunction|AddDialogue "Gardener" "Well, any scraps or expired food! They are easy to decompose, so we compost these wastes into fertilizers." (Utilities|Array|MakeArray "What's an RDF trash?")))
                              (switch Utilities|FlowControl|Switch|SwitchonEnum_DialogueState _state_6
                                (:NewEnumerator0
                                  (switch int _optionindex_6
                                    (:0
                                      (bind (_state_7 _optionindex_7) (CallFunction|AddDialogue "Gardener" "Oh, it's a type of trashes that's hard to decompose and not really worth recycling, so we burn them for energy instead! " (Utilities|Array|MakeArray "Thanks")))
                                      (switch Utilities|FlowControl|Switch|SwitchonEnum_DialogueState _state_7
                                        (:NewEnumerator0
                                          (switch int _optionindex_7
                                            (:0
                                              _))))))))))
                          (bind _state_8 (CallFunction|AddDialogue "Gardener" "Yeah, no problem! See you around!" (Utilities|Array|MakeArray)))
                          (switch Utilities|FlowControl|Switch|SwitchonEnum_DialogueState _state_8
                            (:NewEnumerator0
                              (CallFunction|SetDialogueBranch "AlreadyTalk" "NewEnumerator0")
                              (CallFunction|CloseConversation))))))))))))))
    (:AlreadyTalk
      (bind _state_9 (CallFunction|AddDialogue "Gardener" "You got any trashes on you? Don't forget! Food waste goes into the compost tumbler and RDF goes into the incinerator." (Utilities|Array|MakeArray)))
      (switch Utilities|FlowControl|Switch|SwitchonEnum_DialogueState _state_9
        (:NewEnumerator0
          (CallFunction|ClearDialogueProgress)
          (CallFunction|CloseConversation))))))