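; Dialogue component for the postman NPC, who greets the house's new owner in Thai, explains the mercury hazard of fluorescent bulbs and offers to take them for disposal.
; The Dialogue override calls its parent, then switches on ActiveDialogueBranch.
; The default branch chains AddDialogue lines, some with a single player reply, then sets the AlreadyTalk branch and closes.
; AlreadyTalk shows a short offer of help, clears progress and closes.
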(fn Dialogue
  (|CallParentFunction)
  (switch name (Variables|Default|GetActiveDialogueBranch)
    (:Default
      (bind (_state _optionindex) (CallFunction|AddDialogue "บุรุษไปรษณีย์" "สวัสดีครับ ผมมีจดหมายมาส่งให้คุณน่ะครับ                     " (Utilities|Array|MakeArray)))
      (switch Utilities|FlowControl|Switch|SwitchonEnum_DialogueState _state
        (:NewEnumerator0
          (switch int _optionindex
            (:0
              (bind (_state_2 _optionindex_2) (CallFunction|AddDialogue "บุรุษไปรษณีย์" "คุณคงเป็นเจ้าของคนใหม่ของบ้านหลังสินะ ดูเหมือนว่าคุณกำลังทำความสะอาดบ้านอยู่ใช่มั้ยครับ 
" (Utilities|Array|MakeArray "ใช่แล้ว")))
              (switch Utilities|FlowControl|Switch|SwitchonEnum_DialogueState _state_2
                (:NewEnumerator0
                  (switch int _optionindex_2
                    (:0
                      (bind (_state_3 _optionindex_3) (CallFunction|AddDialogue "บุรุษไปรษณีย์" "เหมือนว่าในบ้านคุณจะมีขยะที่เป็นหลอดไฟด้วย  ถ้าผมจำไม่ผิดร้านรับซื้อขยะไม่รับขยะอันตรายแบบหลอดไฟซะด้วยสิ" (Utilities|Array|MakeArray "ทำไมหลอดไฟถึงอันตรายล่ะ?")))
                      (switch Utilities|FlowControl|Switch|SwitchonEnum_DialogueState _state_3
                        (:NewEnumerator0
                          (switch int _optionindex_3
                            (:0
                              (bind (_state_4 _optionindex_4) (CallFunction|AddDialogue "บุรุษไปรษณีย์" "หืม? ทำไมหลอดไฟถึงอันตรายหรอ? ภายในหลอดไฟฟลูออเรสเซนต์มีสารปรอท ถ้าเกิดแตกขึ้นมาก็จะเกิดอันตรายกับตัวเราเอง อย่าใช้มือเปล่าจับมันเด็ดขาด                                                 " (Utilities|Array|MakeArray)))
                              (switch Utilities|FlowControl|Switch|SwitchonEnum_DialogueState _state_4
                                (:NewEnumerator0
                                  (switch int _optionindex_4
                                    (:0
                                      (bind (_state_5 _optionindex_5) (CallFunction|AddDialogue "บุรุษไปรษณีย์" "แต่คุณไม่ต้องกังวัลนะครับ ผมพอที่จะรู้จักหน่วยงานที่จัดการกับขยะพวกนี้ได้ คุณสามารถฝากหลอดไฟพวกนี้ไว้ที่ผมได้เลย ผมสามารถนำขยะพวกนี้ไปให้พวกเขากำจัดได้" (Utilities|Array|MakeArray "ฝากด้วยนะ")))
                                      (switch Utilities|FlowControl|Switch|SwitchonEnum_DialogueState _state_5
                                        (:NewEnumerator0
                                          (switch int _optionindex_5
                                            (:0
                                              (bind _state_6 (CallFunction|AddDialogue "บุรุษไปรษณีย์" "ไม่ต้องห่วงครับ ผมจะยืนรออยู่ที่หน้าบ้านคุณ ถ้าคุณเจอหลอดไฟเพิ่มเติมก็เอามาให้ผมได้เลยครับ                                           " (Utilities|Array|MakeArray)))
                                              (switch Utilities|FlowControl|Switch|SwitchonEnum_DialogueState _state_6
                                                (:NewEnumerator0
                                                  (CallFunction|SetDialogueBranch "AlreadyTalk" "NewEnumerator0")
                                                  (CallFunction|CloseConversation))))))))))))))))))))))))
    (:AlreadyTalk
      (bind _state_7 (CallFunction|AddDialogue "บุรุษไปรษณีย์" "มีอะไรให้ช่วยมั้ยครับฦ                       " (Utilities|Array|MakeArray)))
      (switch Utilities|FlowControl|Switch|SwitchonEnum_DialogueState _state_7
        (:NewEnumerator0
          (CallFunction|ClearDialogueProgress)
          (CallFunction|CloseConversation))))))