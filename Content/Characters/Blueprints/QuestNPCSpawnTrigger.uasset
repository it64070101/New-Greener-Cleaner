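; QuestNPCSpawnTrigger is a one-shot trigger that brings quest NPCs into the level when the player overlaps its TrashCollision component.
; It shows a notification widget, then spawns actors at the artist, soda maker and terrarium maker spawner markers, each found by class.
; The artist spawn call has no class set in the graph, unlike the other two.
; The trigger destroys itself afterwards.
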(event OnComponentBeginOverlap(TrashCollision)
  (params (OverlappedComponent :type Primitive%20Component%20Object%20Reference) (OtherActor :type Actor%20Object%20Reference) (OtherComp :type Primitive%20Component%20Object%20Reference) (OtherBodyIndex :type Integer) (bFromSweep :type Boolean) (SweepResult :type Hit%20Result%20Structure%20%28by%20ref%29))
  (if (== OtherActor (Game|GetPlayerCharacter 0))
    (bind _returnvalue (UserInterface|CreateWidget "/Game/Inventory/UI/W_Notification.W_Notification_C" 0 "/Game/Inventory/UI/questNPCNotifs.questNPCNotifs"))
    (UserInterface|Viewport|AddtoViewport _returnvalue 0)
    (bind _returnvalue_2 (Actor|GetActorOfClass "/Game/Characters/Artist/BP_ArtistSpawner.BP_ArtistSpawner_C"))
    (Game|SpawnActorfromClass "/Game/Characters/Artist/NPC_Artist.NPC_Artist_C" (Transformation|GetActorTransform _returnvalue_2) "AdjustIfPossibleButAlwaysSpawn" "MultiplyWithRoot" 0 0)
    (bind _returnvalue_3 (Actor|GetActorOfClass "/Game/Characters/SodaMaker/BP_SodaMakerSpawner.BP_SodaMakerSpawner_C"))
    (Game|SpawnActorfromClass "/Game/Characters/SodaMaker/NPC_SodaMaker.NPC_SodaMaker_C" (Transformation|GetActorTransform _returnvalue_3) "Undefined" "MultiplyWithRoot" 0 0)
    (bind _returnvalue_4 (Actor|GetActorOfClass "/Game/Characters/TerrariumMaker/BP_TerraMakerSpawner.BP_TerraMakerSpawner_C"))
    (Game|SpawnActorfromClass "/Game/Characters/TerrariumMaker/NPC_TerrariumMaker.NPC_TerrariumMaker_C" (Transformation|GetActorTransform _returnvalue_4) "Undefined" "MultiplyWithRoot" 0 0)
    (Actor|DestroyActor)))

(fn ConstructionScript)